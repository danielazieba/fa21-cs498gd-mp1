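; BP_TunnelSpawner builds the chain of BP_Tunnel segments around the player.
; On BeginPlay it destroys existing tunnels, then spawns three, starting at the player's location and chaining each to the newest tunnel's SpawnPoint.
; Each spawn gets a spawner reference, a randomized wall and one of six color materials by index modulo.
; SpawnTunnelAtSpawnPoint ignores its MaterialIndex input and uses BP_Player's TunnelIndex instead.
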(event EventBeginPlay
  (CallFunction|SpawnInitialTunnels))

(event Collision|EventActorBeginOverlap
  (params (OtherActor :type Actor%20Object%20Reference)))

(event EventTick
  (params (DeltaSeconds :type Float%20%28single-precision%29)))

(fn ConstructionScript)

(fn SpawnTunnel
  (params (SpawnLocation :type Vector) (MaterialIndex :type Integer))
  (bind _returnvalue (Math|Integer|%(Integer) MaterialIndex 6))
  (bind _returnvalue_2 (Game|SpawnActorfromClass "/Game/InfiniteMatrix/Blueprints/BP_Tunnel.BP_Tunnel_C" (Math|Transform|MakeTransform SpawnLocation "0, 0, 0" "1,1,1") "Undefined" 0 0))
  (bind _output_get (Variables|Default|SetNewestTunnel _returnvalue_2))
  (Variables|/Game/InfiniteMatrix/Blueprints/BP_Tunnel.BP_Tunnel_C|SetTunnelSpawner _output_get self)
  (Default|RandomizeWall _output_get)
  (if (== _returnvalue 0)
    (Rendering|Material|SetMaterial (Variables|/Script/Engine.StaticMeshActor|GetStaticMeshComponent _returnvalue_2) 0 "/Game/InfiniteMatrix/Materials/MI_Tunnel_Red.MI_Tunnel_Red")
    (elif (== _returnvalue 1)
      (Rendering|Material|SetMaterial (Variables|/Script/Engine.StaticMeshActor|GetStaticMeshComponent _returnvalue_2) 0 "/Game/InfiniteMatrix/Materials/MI_Tunnel_Orange.MI_Tunnel_Orange")
      (elif (== _returnvalue 2)
        (Rendering|Material|SetMaterial (Variables|/Script/Engine.StaticMeshActor|GetStaticMeshComponent _returnvalue_2) 0 "/Game/InfiniteMatrix/Materials/MI_Tunnel_Yellow.MI_Tunnel_Yellow")
        (elif (== _returnvalue 3)
          (Rendering|Material|SetMaterial (Variables|/Script/Engine.StaticMeshActor|GetStaticMeshComponent _returnvalue_2) 0 "/Game/InfiniteMatrix/Materials/MI_Tunnel.MI_Tunnel")
          (elif (== _returnvalue 4)
            (Rendering|Material|SetMaterial (Variables|/Script/Engine.StaticMeshActor|GetStaticMeshComponent _returnvalue_2) 0 "/Game/InfiniteMatrix/Materials/MI_Tunnel_Blue.MI_Tunnel_Blue")
            (elif (== _returnvalue 5)
              (Rendering|Material|SetMaterial (Variables|/Script/Engine.StaticMeshActor|GetStaticMeshComponent _returnvalue_2) 0 "/Game/InfiniteMatrix/Materials/MI_Tunnel_Purple.MI_Tunnel_Purple"))))))))

(fn SpawnTunnelatSpawnPoint
  (params (MaterialIndex :type Integer))
  (bind _asbp_player (Utilities|Casting|CastToBP_Player (Game|Player|GetPlayerPawn 0)))
  (CallFunction|SpawnTunnel (Transformation|GetWorldLocation (Variables|/Game/InfiniteMatrix/Blueprints/BP_Tunnel.BP_Tunnel_C|GetSpawnPoint (Variables|Default|GetNewestTunnel))) (Variables|/Game/InfiniteMatrix/Blueprints/BP_Player.BP_Player_C|GetTunnelIndex _asbp_player)))

(fn SpawnInitialTunnels
  (Utilities|FlowControl|Sequence
    (:then_0
      (bind _outactors (Actor|GetAllActorsOfClass "/Game/InfiniteMatrix/Blueprints/BP_Tunnel.BP_Tunnel_C"))
      (for _array_element _outactors
        (Actor|DestroyActor _array_element)))
    (:then_1
      (for _index (range 0 2)
        (Utilities|IsValid (Variables|Default|GetNewestTunnel)
          (:Is%20Valid
            (CallFunction|SpawnTunnelatSpawnPoint _index))
          (:Is%20Not%20Valid
            (CallFunction|SpawnTunnel (Transformation|GetActorLocation (Game|Player|GetPlayerPawn 0)) _index)))))))